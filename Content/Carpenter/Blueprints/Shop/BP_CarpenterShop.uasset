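; BP_CarpenterShop is the carpenter shop actor that hosts chipper and painter workbenches as child actor components.
; On BeginPlay it assigns the chipper's child actor class at runtime, while the painter relies on its existing child actor.
; It casts each child actor to its workbench Blueprint and passes itself as the owning shop, giving both benches a back-reference.
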(event `self.ReceiveBeginPlay`
  (`|ExecutionSequence`
    (:`then_0`
      (`ChildActorComponent.SetChildActorClass` (`self.ChipperWorkbench`) "/Game/Carpenter/Blueprints/Shop/Workbenches/BP_WorkbenchChipper.BP_WorkbenchChipper_C")
      (bind _asbp_workbench_chipper (cast `/Game/Carpenter/Blueprints/Shop/Workbenches/BP_WorkbenchChipper` (`ChildActorComponent.ChildActor` (`self.ChipperWorkbench`))))
      (`CarpenterWorkbenchBase.SetOwningCarpenterShop` _asbp_workbench_chipper self))
    (:`then_1`
      (bind _asbp_workbench_painter (cast `/Game/Carpenter/Blueprints/Shop/Workbenches/BP_WorkbenchPainter` (`ChildActorComponent.ChildActor` (`self.PainterWorkbench`))))
      (`CarpenterWorkbenchBase.SetOwningCarpenterShop` _asbp_workbench_painter self))))

(fn `UserConstructionScript`)