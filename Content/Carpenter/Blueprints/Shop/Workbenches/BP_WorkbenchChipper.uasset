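; BP_WorkbenchChipper is the chipper workbench in the carpenter workshop shop, operated through a left and a right button.
; On BeginPlay it casts each button's child actor to CarpenterWorkshopButtonBase and binds its OnButtonInteracted event to a matching click handler.
; Both handlers only forward to the parent class, so the actual button behavior is inherited rather than defined here.
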(event `self.ReceiveBeginPlay`
  (`|ExecutionSequence`
    (:`then_0`
      (bind _ascarpenter_workshop_button_base (cast `CarpenterWorkshopButtonBase` (`ChildActorComponent.ChildActor` (`self.LeftButton`))))
      (add `CarpenterWorkshopButtonBase.OnButtonInteracted` _ascarpenter_workshop_button_base (delegate `self.LeftButtonClicked`)))
    (:`then_1`
      (bind _ascarpenter_workshop_button_base_2 (cast `CarpenterWorkshopButtonBase` (`ChildActorComponent.ChildActor` (`self.RightButton`))))
      (add `CarpenterWorkshopButtonBase.OnButtonInteracted` _ascarpenter_workshop_button_base_2 (delegate `self.RightButtonClicked`)))))

(event `self.LeftButtonClicked`
  (`parent.LeftButtonClicked`))

(event `self.RightButtonClicked`
  (`parent.RightButtonClicked`))

(fn `UserConstructionScript`)